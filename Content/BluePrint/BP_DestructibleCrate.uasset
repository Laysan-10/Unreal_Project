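; BP_DestructibleCrate is a crate Blueprint meant to lose health from damage and be destroyed, though that logic is unfinished.
; An EventGraph chain, unconnected to any event so it never runs, subtracts Damage from Health, then either prints and destroys the actor or prints the remaining health.
; ApplyDamage, GetHealth and IsDestroyed are stubs returning false or zero, and the construction script is empty.
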(fn ConstructionScript)

(fn ApplyDamage
  (params (DamageAmount :type Float%20%28double-precision%29))
  (return false))

(fn GetHealth
  (return 0.0))

(fn IsDestroyed
  (return false))