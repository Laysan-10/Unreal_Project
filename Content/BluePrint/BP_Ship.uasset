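; Flyable physics ship that the first-person player enters via interaction and leaves via input, toggling its thruster.
; Lift comes from a mass-scaled, tilt-compensated physics thruster, with center of mass shifted to its XY position at BeginPlay.
; Throttle input eases forward thrust, which drives engine RPM audio and, above a threshold, overrides linear velocity each tick.
; Pitch, yaw and roll apply torque only above that threshold, while lift input works only below a higher one.
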(event Custom|OnShipUnoccupied
  ;[1 1 1] Set ship unoccupied
  (Variables|Default|SetOnShipOccupied false)
  (Variables|/Game/FirstPerson/Blueprints/BP_FirstPersonCharacter.BP_FirstPersonCharacter_C|SetCurrentShip (Variables|Default|GetPlayer) 0)
  (Components|Activation|Deactivate (Variables|Default|GetPhysicsThruster)))

(event Input|EnhancedActionEvents|EnhancedInputActionIA_LeaveShip
  (params (ActionValue :type Boolean) (ElapsedSeconds :type Float%20%28double-precision%29) (TriggeredSeconds :type Float%20%28double-precision%29) (InputAction :type Input%20Action%20Object%20Reference :default "/Game/Input_Action/IA_LeaveShip.IA_LeaveShip"))
  ;[1 1 1] Leave ship
  (:Started
    (Default|OnShipLeave (Variables|Default|GetPlayer))
    (Audio|Parameter|SetFloatParameter (Variables|Default|GetAudioCurveSource) "RPM" 0.0 :!class /Script/Engine.AudioComponent)))

(event Input|EnhancedActionEvents|EnhancedInputActionIA_Fly
  (params (ActionValue :type Float%20%28double-precision%29) (ElapsedSeconds :type Float%20%28double-precision%29) (TriggeredSeconds :type Float%20%28double-precision%29) (InputAction :type Input%20Action%20Object%20Reference :default "/Game/Input_Action/IA_Fly.IA_Fly"))
  (bind _physicsthruster (Variables|Default|GetPhysicsThruster))
  (:Triggered
    (if (<= (Variables|Default|GetForwardThrust) 3e+03)
      (Variables|/Script/Engine.PhysicsThrusterComponent|SetThrustStrength _physicsthruster (* (/ (* ActionValue (Variables|Default|GetUpDownthrustStrength)) (.z (Transformation|GetActorUpVector))) (Physics|GetMass (Variables|Default|GetCube))))))
  (:Completed
    (Variables|/Script/Engine.PhysicsThrusterComponent|SetThrustStrength _physicsthruster 0.0)))

(event Input|EnhancedActionEvents|EnhancedInputActionIA_UpDownMouseShipControl
  (params (ActionValue :type Float%20%28double-precision%29) (ElapsedSeconds :type Float%20%28double-precision%29) (TriggeredSeconds :type Float%20%28double-precision%29) (InputAction :type Input%20Action%20Object%20Reference :default "/Game/Input_Action/IA_UpDownMouseShipControl.IA_UpDownMouseShipControl"))
  (:Triggered
    (CallFunction|RotateShip (Math|Vector|GetRightVector (Variables|Default|GetCube)) (Variables|Default|GetUpdownTorqueStraiht) ActionValue)))

(event Input|EnhancedActionEvents|EnhancedInputActionIA_LeftRightShipControl
  (params (ActionValue :type Float%20%28double-precision%29) (ElapsedSeconds :type Float%20%28double-precision%29) (TriggeredSeconds :type Float%20%28double-precision%29) (InputAction :type Input%20Action%20Object%20Reference :default "/Game/Input_Action/IA_LeftRightShipControl.IA_LeftRightShipControl"))
  (:Triggered
    (CallFunction|RotateShip (Math|Vector|GetUpVector (Variables|Default|GetCube)) (Variables|Default|GetLeftRightTorqueStraight) ActionValue)))

(event Input|EnhancedActionEvents|EnhancedInputActionIA_RollShipContol
  (params (ActionValue :type Float%20%28double-precision%29) (ElapsedSeconds :type Float%20%28double-precision%29) (TriggeredSeconds :type Float%20%28double-precision%29) (InputAction :type Input%20Action%20Object%20Reference :default "/Game/Input_Action/IA_RollShipContol.IA_RollShipContol"))
  (:Triggered
    (CallFunction|RotateShip (Math|Vector|GetForwardVector (Variables|Default|GetCube)) (Variables|Default|GetRollTorqueStraight) ActionValue)))

(event Input|EnhancedActionEvents|EnhancedInputActionIA_ForwardBackwardShip
  (params (ActionValue :type Float%20%28double-precision%29) (ElapsedSeconds :type Float%20%28double-precision%29) (TriggeredSeconds :type Float%20%28double-precision%29) (InputAction :type Input%20Action%20Object%20Reference :default "/Game/Input_Action/IA_ForwardBackwardShip.IA_ForwardBackwardShip"))
  (:Triggered
    (Utilities|FlowControl|Sequence
      (:then_0
        (if (>= ActionValue 0.0)
          (Variables|Default|SetTargetLerpAlpha 1.0)
          (else
            (Variables|Default|SetTargetLerpAlpha 0.0)))
        (bind _output_get (Variables|Default|SetForwardThrust (Math|Interpolation|FInterpTo (Variables|Default|GetForwardThrust) (Math|Float|Lerp 0.0 (Variables|Default|GetMaxForwardThrust) (Variables|Default|GetTargetLerpAlpha)) (Utilities|Time|GetWorldDeltaSeconds) 0.0)))
        (Audio|Parameter|SetFloatParameter (Variables|Default|GetAudioCurveSource) "RPM" (Math|Float|MapRangeClamped (Math|Float|Absolute(Float) _output_get) 0.0 (Variables|Default|GetMaxForwardThrust) 0.0 1.0) :!class /Script/Engine.AudioComponent))
      (:then_1
        (Variables|Default|SetForwardMoveVector (* (Math|Vector|GetForwardVector (Variables|Default|GetCube)) (Variables|Default|GetForwardThrust)))))))

(event EventBeginPlay
  (bind _physicsthruster (Variables|Default|GetPhysicsThruster))
  (bind _cube (Variables|Default|GetCube))
  (bind _returnvalue (Transformation|GetWorldLocation _physicsthruster))
  (bind _returnvalue_2 (Physics|GetCenterOfMass _cube "None"))
  (bind _returnvalue_3 (Transformation|GetWorldRotation _cube))
  (bind _returnvalue_4 (Class|KismetMathLibrary|NegateRotator _returnvalue_3))
  (bind _returnvalue_5 (- _returnvalue _returnvalue_2))
  (bind _returnvalue_6 (Math|Vector|RotateVector _returnvalue_5 _returnvalue_4))
  ;[1 1 1] Get Player (Initialization)
  (bind _asbp_first_person_character (Utilities|Casting|CastToBP_FirstPersonCharacter (Game|GetPlayerCharacter 0)))
  (Variables|Default|SetPlayer _asbp_first_person_character)
  (Variables|Default|SetShipStaticMesh (Variables|Default|GetCube))
  (Class|PrimitiveComponent|SetCenterOfMass (Variables|Default|GetCube) (Math|Vector|MakeVector (.x _returnvalue_6) (.y _returnvalue_6) 0.0) "None")
  (Audio|Parameter|SetFloatParameter (Variables|Default|GetAudioCurveSource) "RPM" 0.0 :!class /Script/Engine.AudioComponent))

(event EventTick
  (params (DeltaSeconds :type Float%20%28single-precision%29))
  ;[1 1 1] Move Forward
  (if (>= (Variables|Default|GetForwardThrust) 2e+02)
    (Physics|SetPhysicsLinearVelocity (Variables|Default|GetCube) (Variables|Default|GetForwardMoveVector) false "None")))

(event EventInteract
  (bind _player (Variables|Default|GetPlayer))
  ;[1 1 1] Interact with ship
  (Development|PrintString "Interact")
  (if (not (Variables|Default|GetOnShipOccupied))
    (Variables|Default|SetOnShipOccupied true)
    (Variables|/Game/FirstPerson/Blueprints/BP_FirstPersonCharacter.BP_FirstPersonCharacter_C|SetCurrentShip _player self)
    (Default|OnShipOccupied _player)
    (Components|Activation|Activate (Variables|Default|GetPhysicsThruster) false)
    (Audio|Parameter|SetFloatParameter (Variables|Default|GetAudioCurveSource) "RPM" (Math|Float|MapRangeClamped (Math|Float|Absolute(Float) (Variables|Default|GetForwardThrust)) 0.0 (Variables|Default|GetMaxForwardThrust) 0.0 1.0) :!class /Script/Engine.AudioComponent)))

(fn ConstructionScript)

(fn RotateShip
  (params (Origin :type Vector) (Torque%20Value :type Float%20%28double-precision%29) (Input%20Value :type Float%20%28double-precision%29))
  (if (>= (Variables|Default|GetForwardThrust) 2e+02)
    (Class|PrimitiveComponent|AddTorqueinDegrees (Variables|Default|GetCube) (* Origin (* Torque%20Value Input%20Value)) "None" true)))